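; BP_Fur is an actor that renders shell-style fur on a configurable mesh by stacking layered copies of it.
; On BeginPlay it sets the base StaticMesh, then calls CreateLayer repeatedly with evenly stepped offsets from zero to one.
; Each call adds a static mesh component with a dynamic Fur_Inst material whose FUR_OFFSET parameter receives that layer's offset.
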(event `Create Layer`
  (params (FUR_OFFSET :type "Float (double-precision)"))
  (bind _returnvalue (`AddComponent|NODE_AddStaticMeshComponent-4`))
  (bind _output_get (set `self.MeshComponent` _returnvalue))
  (`StaticMeshComponent.SetStaticMesh` _output_get (`self.Mesh`))
  (bind _returnvalue_2 (`PrimitiveComponent.CreateDynamicMaterialInstance` _output_get 0 "/Game/Fur_Inst.Fur_Inst" "None"))
  (`MaterialInstanceDynamic.SetScalarParameterValue` _returnvalue_2 "FUR_OFFSET" FUR_OFFSET))

(event `self.ReceiveBeginPlay`
  (`StaticMeshComponent.SetStaticMesh` (`self.StaticMesh`) (`self.Mesh`))
  (`self.Create Layer` 0.0)
  (`self.Create Layer` 0.05)
  (`self.Create Layer` 0.1)
  (`self.Create Layer` 0.15)
  (`self.Create Layer` 0.2)
  (`self.Create Layer` 0.25)
  (`self.Create Layer` 0.3)
  (`self.Create Layer` 0.35)
  (`self.Create Layer` 0.4)
  (`self.Create Layer` 0.45)
  (`self.Create Layer` 0.5)
  (`self.Create Layer` 0.55)
  (`self.Create Layer` 0.6)
  (`self.Create Layer` 0.65)
  (`self.Create Layer` 0.7)
  (`self.Create Layer` 0.75)
  (`self.Create Layer` 0.8)
  (`self.Create Layer` 0.85)
  (`self.Create Layer` 0.9)
  (`self.Create Layer` 0.95)
  (`self.Create Layer` 1.0))

(fn `UserConstructionScript`)